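; BP_DoorFrame is a door frame actor that shows one randomly chosen door out of four and animates its vertical position when play begins.
; BeginPlay hides all four door components, then unhides a random one.
; The timeline Zeitleiste then drives the root component's height with a swept move, scaling its track value and pinning X and Y to hardcoded world coordinates rather than the placed location.
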(event EventBeginPlay
  (bind _door (Variables|Default|GetDoor))
  (bind _door1 (Variables|Default|GetDoor1))
  (bind _door2 (Variables|Default|GetDoor2))
  (bind _door3 (Variables|Default|GetDoor3))
  (bind _array (Utilities|Array|MakeArray _door _door1 _door2 _door3))
  (for _array_element _array
    (Development|SetHiddeninGame _array_element true false))
  (Development|SetHiddeninGame (.OutItem (Utilities|Array|Random _array)) false false)
  (bind _neuer_track_0 (Timeline|Zeitleiste Play)
    (:Update
      (Transformation|SetWorldLocation (Variables|Default|GetDefaultSceneRoot) (Math|Vector|MakeVector 1.5e+02 -4e+01 (* _neuer_track_0 3e+02)) true false))))

(fn ConstructionScript)