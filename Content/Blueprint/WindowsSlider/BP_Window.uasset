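; BP_Window is a Paper2D sprite actor that repeatedly slides along its relative X axis on a timeline.
; InitObject stores an Offset and waits that many seconds before calling MoveObject, so the start can be staggered.
; Each timeline update scales the track to set the X position and snaps the sprite between 0 and 180 degrees rotation at a position threshold.
; When the timeline finishes, it restarts after a fixed delay.
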(event Custom|InitObject
  (params (Offset :type Float%20%28double-precision%29))
  (bind _output_get (Variables|Default|Setoffset Offset))
  (Utilities|FlowControl|Delay _output_get)
  (CallFunction|MoveObject))

(event Custom|MoveObject
  (bind _papersprite (Variables|Default|GetPaperSprite))
  (bind _relativelocation (Variables|/Script/Engine.SceneComponent|GetRelativeLocation _papersprite))
  (bind _newtrack_0 (Timeline|Timeline PlayFromStart)
    (:Update
      (if (< (* _newtrack_0 5e+02) 2.5e+02)
        (Transformation|SetRelativeRotation (Variables|Default|GetPaperSprite) "0, 0, 0" false false)
        (else
          (Transformation|SetRelativeRotation (Variables|Default|GetPaperSprite) "0.000000,180.000000,0.000000" false false)))
      (Transformation|SetRelativeLocation (Variables|Default|GetPaperSprite) (Math|Vector|MakeVector (* _newtrack_0 5e+02) (.y _relativelocation) (.z _relativelocation)) false false))
    (:Finished
      (Utilities|FlowControl|Delay 7.0)
      (Timeline|Timeline PlayFromStart))))

(fn ConstructionScript)